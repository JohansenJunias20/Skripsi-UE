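; Shared VR whiteboard actor that paints marker strokes onto a render target through a dynamic material.
; Start, draw and release events let one user draw at a time, identified according to the EOS or CICE network mode.
; Incoming points form chained three-point quadratic Bezier curves, stamped by repeatedly drawing the material to the target.
; The tools widget's clear event wipes the board and sends the clear over the active network.
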(event `onClearWhiteboard`
  (`|ExecutionSequence`
    (:`then_0`
      (`KismetRenderingLibrary.ClearRenderTarget2D` "/Game/WhiteBoard/CRT_Whiteboard.CRT_Whiteboard" :!label _label))
    (:`then_1`
      (bind _asblueprint_gi (cast `/Game/BlueprintGI` (`GameplayStatics.GetGameInstance`)))
      (switch `/Game/Enums/Enum_NetworkMode` (`/Game/BlueprintGI.NetworkMode` _asblueprint_gi)
        (:`NewEnumerator0`
          (bind _asbp_vrcharacter (cast `/Game/BP_VRCharacter` (`GameplayStatics.GetPlayerCharacter` 0)))
          (bind _returnvalue (`/Game/Functions/utilities.getUnixTimestamp`))
          (`/Game/BP_VRCharacter.ClearWhiteboardServer` _asbp_vrcharacter _returnvalue))
        (:`NewEnumerator1`
          (`/Game/BlueprintGI.ED_SendReliableData` _asblueprint_gi null "NewEnumerator1" "" "NewEnumerator19"))))))

(event `ClearWhiteBoardSignal`
  (`MaterialInstanceDynamic.SetScalarParameterValue` (`self.WhiteboardMarker_Ml`) "DrawSize" 0.0)
  (`KismetRenderingLibrary.DrawMaterialToRenderTarget` "/Game/WhiteBoard/CRT_Whiteboard.CRT_Whiteboard" (`self.WhiteboardMarker_Ml`))
  (`KismetSystemLibrary.DelayUntilNextTick`)
  (goto _label))

(event `self.ReceiveBeginPlay`
  (`|ExecutionSequence`
    (:`then_0`
      (bind _aswb_whiteboard_tools (cast `/Game/WhiteBoard/WB_WhiteboardTools` (`WidgetComponent.GetUserWidgetObject` (`self.Widget Whiteboard`))))
      (add `/Game/WhiteBoard/WB_WhiteboardTools.onClear` _aswb_whiteboard_tools (delegate `onClearWhiteboard`))
      (bind _returnvalue (`KismetMaterialLibrary.CreateDynamicMaterialInstance` "/Game/WhiteBoard/M_WhiteboardMarker.M_WhiteboardMarker"))
      (set `self.WhiteboardMarker_Ml` _returnvalue)
      (`KismetRenderingLibrary.ClearRenderTarget2D` "/Game/WhiteBoard/CRT_Whiteboard.CRT_Whiteboard"))
    (:`then_1`
      (bind _asblueprint_gi (cast `/Game/BlueprintGI` (`GameplayStatics.GetGameInstance`)))
      (set `/Game/BlueprintGI.whiteboardRef` self _asblueprint_gi)
      (set `self.as GI` _asblueprint_gi))))

(event `StartWhiteBoard`
  (params (socketio_id :type String) (id :type Integer))
  (if (not (`self.isDrawing?`))
    (switch `/Game/Enums/Enum_NetworkMode` (`/Game/BlueprintGI.NetworkMode` (cast `/Game/BlueprintGI` (`GameplayStatics.GetGameInstance`) :!pure true))
      (:`NewEnumerator0`
        (set `self.EOSdrawingBy?` id))
      (:`NewEnumerator1`
        (set `self.CICEdrawingBy?` socketio_id)))
    (set `self.isDrawing?` true)
    (`KismetSystemLibrary.PrintString` "IS DRAWING IS SET TO TRUE")
    (else
      (`KismetSystemLibrary.PrintString` "CANNOT DRAW, DRAW BY SOMEONE ELSE" true true (struct :`R` 1.0 :`B` 0.042729 :`A` 1.0) 5.0))))

(event `Draw On WhiteBoard`
  (params (NewParam :type "Vector2D Structure") (byEOS :type Integer) (byCICE :type String))
  (bind _3points (`self.3points`))
  (if (`self.isDrawing?`)
    (switch `/Game/Enums/Enum_NetworkMode` (`/Game/BlueprintGI.NetworkMode` (cast `/Game/BlueprintGI` (`GameplayStatics.GetGameInstance`) :!pure true))
      (:`NewEnumerator0`
        (if (== (`self.EOSdrawingBy?`) byEOS)
          (`KismetArrayLibrary.Array_Add` _3points NewParam :!label _label_2)
          (if (== (`KismetArrayLibrary.Array_Length` _3points) 3)
            (`self.3DrawBezier`)
            (`KismetArrayLibrary.Array_Remove` _3points)
            (`KismetArrayLibrary.Array_Remove` _3points))))
      (:`NewEnumerator1`
        (if (`KismetStringLibrary.EqualEqual_StrStr` (`self.CICEdrawingBy?`) byCICE)
          (goto _label_2))))
    (else
      (`KismetSystemLibrary.PrintString` "IS DRAWINGGGGG..."))))

(event `release whiteboard`
  (params (EOSby :type Integer) (CICEby :type String))
  (if (`self.isDrawing?`)
    (switch `/Game/Enums/Enum_NetworkMode` (`/Game/BlueprintGI.NetworkMode` (cast `/Game/BlueprintGI` (`GameplayStatics.GetGameInstance`) :!pure true))
      (:`NewEnumerator0`
        (if (== EOSby (`self.EOSdrawingBy?`))
          (set `self.EOSdrawingBy?` -1)
          (`KismetArrayLibrary.Array_Clear` (`self.3points`) :!label _label_3)
          (set `self.isDrawing?` false)
          (`KismetSystemLibrary.PrintString` "REMOVING DRAWING BY" true true (struct :`R` 1.0 :`B` 0.078098 :`A` 1.0) 5.0)
          (`KismetSystemLibrary.PrintString` "REMOVING DRAWING BY" true true (struct :`R` 1.0 :`B` 0.078098 :`A` 1.0) 5.0)))
      (:`NewEnumerator1`
        (if (`KismetStringLibrary.EqualEqual_StrStr` CICEby (`self.CICEdrawingBy?`))
          (set `self.CICEdrawingBy?` "")
          (goto _label_3))))
    (else
      (`KismetSystemLibrary.PrintString` "IS NOT DRAWING.. (RELEASE)"))))

(fn `3DrawBezier`
  (locals (t :type "Float (double-precision)") (numberDrawPoints :type Integer :default 30) (x :type "Float (double-precision)") (y :type "Float (double-precision)") (controlX :type "Float (double-precision)") (controlY :type "Float (double-precision)"))
  (bind _3points (`self.3points`))
  (bind _whiteboardmarker_ml (`self.WhiteboardMarker_Ml`))
  (bind _numberdrawpoints (`local.numberDrawPoints`))
  (bind (_output_x _output_y) (`KismetMathLibrary.BreakVector2D` (`|GetArrayItem` _3points)))
  (bind (_output_x_2 _output_y_2) (`KismetMathLibrary.BreakVector2D` (`|GetArrayItem` _3points 1)))
  (bind (_output_x_3 _output_y_3) (`KismetMathLibrary.BreakVector2D` (`|GetArrayItem` _3points 2)))
  (`MaterialInstanceDynamic.SetScalarParameterValue` _whiteboardmarker_ml "DrawSize" 0.01)
  (for _index (range (+ _numberdrawpoints 1))
    (bind _output_get (set `local.t` (/ _index _numberdrawpoints)))
    (bind _output_get_2 (set `local.x` (`self.calcBezierPoint` _output_get _output_x _output_x_2 _output_x_3)))
    (bind _output_get_3 (set `local.y` (`self.calcBezierPoint` _output_get _output_y _output_y_2 _output_y_3)))
    (`MaterialInstanceDynamic.SetVectorParameterValue` _whiteboardmarker_ml "DrawLocation" (make `LinearColor` _output_get_2 _output_get_3))
    (`KismetRenderingLibrary.DrawMaterialToRenderTarget` "/Game/WhiteBoard/CRT_Whiteboard.CRT_Whiteboard" _whiteboardmarker_ml)))

(fn `DrawBezier`
  (params (curveStart :type "Vector2D Structure") (curveEnd :type "Vector2D Structure") (numDrawPoints :type "Float (double-precision)"))
  (locals (t :type "Float (double-precision)") (numberDrawPoints :type Integer) (x :type "Float (double-precision)") (y :type "Float (double-precision)") (controlX :type "Float (double-precision)") (controlY :type "Float (double-precision)"))
  (bind _returnvalue (`KismetMathLibrary.FCeil` numDrawPoints))
  (bind _whiteboardmarker_ml (`self.WhiteboardMarker_Ml`))
  (for _index (range (+ _returnvalue 1))
    (bind _output_get (set `local.t` (/ _index _returnvalue)))
    (bind _output_get_2 (set `local.x` (`self.calcBezierPoint` _output_get curveStart_X (`self.findControl` curveStart_X curveEnd_X) curveEnd_X)))
    (bind _output_get_3 (set `local.y` (`self.calcBezierPoint` _output_get curveStart_Y (`self.findControl` curveStart_Y curveEnd_Y) curveEnd_Y)))
    (`MaterialInstanceDynamic.SetVectorParameterValue` _whiteboardmarker_ml "DrawLocation" (make `LinearColor` _output_get_2 _output_get_3))
    (`KismetRenderingLibrary.DrawMaterialToRenderTarget` "/Game/WhiteBoard/CRT_Whiteboard.CRT_Whiteboard" _whiteboardmarker_ml)))

(fn `nDrawBezier`
  (locals (t :type "Float (double-precision)") (numberDrawPoints :type Integer :default 15) (x :type "Float (double-precision)") (y :type "Float (double-precision)") (controlX :type "Float (double-precision)") (controlY :type "Float (double-precision)") (coeff :type "Float (double-precision)"))
  (bind _whiteboardmarker_ml (`self.WhiteboardMarker_Ml`))
  (bind _numberdrawpoints (`local.numberDrawPoints`))
  (`self.ClearWhiteBoardSignal`)
  (`MaterialInstanceDynamic.SetScalarParameterValue` (`self.WhiteboardMarker_Ml`) "DrawSize" 0.01)
  (for _index (range (+ _numberdrawpoints 1))
    (bind _output_get (set `local.t` (/ (`KismetMathLibrary.Conv_IntToDouble` _index) (`KismetMathLibrary.Conv_IntToDouble` _numberdrawpoints))))
    (set `local.x` 0.0)
    (set `local.y` 0.0)
    (for (_array_element _array_index) (`self.points`)
      (bind _returnvalue (`self.calcBinCoeff` _array_index (`local.numberDrawPoints`) _output_get))
      (bind _output_get_2 (set `local.coeff` _returnvalue))
      (set `local.x` (+ (`local.x`) (* _output_get_2 (`KismetMathLibrary.BreakVector2D` _array_element))))
      (set `local.y` (+ (`local.y`) (* _output_get_2 (`.Y` (`KismetMathLibrary.BreakVector2D` _array_element))))))
    (`MaterialInstanceDynamic.SetVectorParameterValue` _whiteboardmarker_ml "DrawLocation" (make `LinearColor` (`local.x`) (`local.y`)))
    (`KismetRenderingLibrary.DrawMaterialToRenderTarget` "/Game/WhiteBoard/CRT_Whiteboard.CRT_Whiteboard" _whiteboardmarker_ml)))

(fn `UserConstructionScript`)