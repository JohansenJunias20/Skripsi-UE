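; Door Blueprint that swings open automatically when a BP_VRCharacter enters its trigger box.
; The box overlap plays the OpenDoor timeline, whose alpha lerps the static mesh's rotation toward a fixed open angle.
; When the last VR character leaves the box, the timeline reverses to close the door.
; The rotation is set in world space, so it does not follow the placed actor's orientation.
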(event `self.Box.OnComponentBeginOverlap`
  (params (OverlappedComponent :type "PrimitiveComponent Object Reference") (OtherActor :type "Actor Object Reference") (OtherComp :type "PrimitiveComponent Object Reference") (OtherBodyIndex :type Integer) (bFromSweep :type Boolean) (SweepResult :type "HitResult Structure (by ref)"))
  (if (== (`GameplayStatics.GetObjectClass` OtherActor) "/Game/BP_VRCharacter.BP_VRCharacter_C")
    (bind (_direction _alpha_lerp) (`Timeline|OpenDoor` :!label _label)
      (:`Update`
        (`SceneComponent.K2_SetWorldRotation` (`self.StaticMesh`) (`KismetMathLibrary.RLerp` (struct) (struct :`Yaw` 105.0) _alpha_lerp true) false false)))))

(event `self.Box.OnComponentEndOverlap`
  (params (OverlappedComponent :type "PrimitiveComponent Object Reference") (OtherActor :type "Actor Object Reference") (OtherComp :type "PrimitiveComponent Object Reference") (OtherBodyIndex :type Integer))
  (if (== (`GameplayStatics.GetObjectClass` OtherActor) "/Game/BP_VRCharacter.BP_VRCharacter_C")
    (if (`KismetArrayLibrary.Array_IsEmpty` (`PrimitiveComponent.GetOverlappingActors` (`self.Box`) "/Game/BP_VRCharacter.BP_VRCharacter_C"))
      (goto _label :!via `Reverse`))))

(fn `UserConstructionScript`)