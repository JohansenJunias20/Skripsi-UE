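; BP_Latency is a stub Blueprint, named for latency, with an empty BeginPlay and construction script.
; Its getUnixTimestamp graph holds an unused node chain that computes UTC milliseconds since 1 January 1970.
; The chain rebuilds the total from the timespan's hour, minute, second and millisecond parts, converting to Int64 after the seconds sum is multiplied to milliseconds.
; No latency measurement is present.
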(event `self.ReceiveBeginPlay`)

(fn `UserConstructionScript`)