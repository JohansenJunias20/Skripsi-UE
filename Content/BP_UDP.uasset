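; BP_UDP is the unreliable UDP transport syncing VR players and whiteboard drawing, opening its sockets once the game instance reports TCP established.
; Outgoing data becomes timestamped JSON bytes; incoming packets are filtered by recipient, then routed by channel.
; Transforms update characters and server tick data, which clients apply to remote avatars and breakout buttons, using Old or New formats per SendMethod.
; The server echoes timestamps, feeding latency statistics in BlueprintGI.
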(event `self.ReceiveBeginPlay`
  (bind _asblueprint_gi (cast `/Game/BlueprintGI` (`GameplayStatics.GetGameInstance`)))
  (add `/Game/BlueprintGI.ED_TCPestablished` _asblueprint_gi (delegate `Start`))
  (add `/Game/BlueprintGI.ED_SendUnreliableData` _asblueprint_gi (delegate `SendUnreliable`))
  ;[1 1 1] recieve UDP p2p message
  (add `UDPComponent.OnReceivedBytes` (`self.UDP`) (delegate `Recieve Bytes`)))

(event `SendUnreliable`
  (params (input :type "SIOJsonObject Object Reference") (to :type "/Game/Enums/Enum_SendTo Enum" :default "NewEnumerator0") (socketid :type String) (channel :type "/Game/Enums/Enum_Channel Enum" :default "NewEnumerator0"))
  (bind _returnvalue (`SIOJsonObject.ConstructJsonObject`))
  (bind _asblueprint_gi (cast `/Game/BlueprintGI` (`GameplayStatics.GetGameInstance`)))
  (`SIOJsonObject.SetStringField` _returnvalue "from" (`/Game/BlueprintGI.socketid` _asblueprint_gi))
  (`SIOJsonObject.SetStringField` _returnvalue "to" (`|GetEnumeratorNameAsString` to))
  (`SIOJsonObject.SetField` _returnvalue "data" (`SIOJLibrary.Conv_JsonObjectToJsonValue` input))
  (`SIOJsonObject.SetStringField` _returnvalue "socketid" socketid)
  (`SIOJsonObject.SetStringField` _returnvalue "channel" (`|GetEnumeratorNameAsString` channel))
  (bind _returnvalue_2 (`/Game/Functions/utilities.getUnixTimestamp`))
  (`SIOJsonObject.SetObjectField` _returnvalue "timestamp" (`SIOJLibrary.StructToJsonObject` (make `/Game/Structs/Struct_Timestamp` _returnvalue_2)))
  (`UDPComponent.EmitBytes` (`self.UDP`) (`CUBlueprintLibrary.Conv_StringToBytes` (`SIOJLibrary.Conv_SIOJsonObjectToString` _returnvalue))))

(event `Recieve Bytes`
  (params (Bytes :type "Array of Byte (by ref)") (IPAddress :type String))
  (bind _returnvalue (`GameplayStatics.GetGameInstance`))
  (bind _asblueprint_gi (cast `/Game/BlueprintGI` (`GameplayStatics.GetGameInstance`) :!pure true))
  (bind _asblueprint_gi_2 (cast `/Game/BlueprintGI` (`GameplayStatics.GetGameInstance`) :!pure true))
  ;[1 1 1] recieve UDP p2p message
  (bind _outjsonobject (`JsonBlueprintFunctionLibrary.FromString` (`CUBlueprintLibrary.Conv_BytesToString` Bytes)))
  (bind _outvalue (`|GetJsonField` _outjsonobject "to"))
  (bind _newparam1 (`/Game/Functions/utilities.StringToEnumSendTo` _outvalue))
  (switch `/Game/Enums/Enum_SendTo` _newparam1
    (:`NewEnumerator0`
      (bind _asblueprint_gi_3 (cast `/Game/BlueprintGI` _returnvalue))
      (if (`|EnumEquality` (`/Game/BlueprintGI.role` _asblueprint_gi_3) "NewEnumerator0")
        (bind _outvalue_2 (`|GetJsonField` _outjsonobject "data" :!label _label))
        (bind _outvalue_3 (`|GetJsonField` _outjsonobject "channel"))
        (switch `string` _outvalue_3
          (:`transform`
            (bind _outvalue_4 (`|GetJsonField` _outvalue_2 "timestamp"))
            (`|ExecutionSequence`
              (:`then_0`
                (`self.replyTimestamp` _outjsonobject)
                ;;[1 1 1] position
                (bind _outvalue_5 (`|GetJsonField` _outvalue_2 "position"))
                ;;;[1 1 1] ini error masih ke set 0,0,0
                (bind (_outvalue_6 _returnvalue_2) (`|GetJsonField` _outvalue_5 "x"))
                (bind _outvalue_7 (`|GetJsonField` _outvalue_5 "y"))
                (bind _outvalue_8 (`|GetJsonField` _outvalue_5 "z"))
                (`self.SwitchSendMethod`
                  (:`Old`
                    (for _array_element (`/Game/BlueprintGI.players_actor` (cast `/Game/BlueprintGI` (`GameplayStatics.GetGameInstance`) :!pure true))
                      (bind _asbp_vrcharacter (cast `/Game/BP_VRCharacter` _array_element))
                      (bind (_outvalue_9 _returnvalue_3) (`|GetJsonField` _outjsonobject "from"))
                      (if (and (`KismetStringLibrary.EqualEqual_StrStr` (`/Game/BP_VRCharacter.socketio_id` _asbp_vrcharacter) _outvalue_9) _returnvalue_3)
                        (bind _returnvalue_4 (`KismetMathLibrary.MakeVector` _outvalue_6 _outvalue_7 _outvalue_8))
                        (`self.K2_SetActorLocation` _array_element _returnvalue_4 false false)
                        (`self.SwitchSendMethod`
                          (:`Old`
                            (bind _outvalue_10 (`|GetJsonField` _outvalue_2 "MC_Left"))
                            (bind _outvalue_11 (`|GetJsonField` _outvalue_2 "MC_Right"))
                            (bind _outvalue_12 (`|GetJsonField` _outvalue_2 "camera"))
                            (set `/Game/BP_VRCharacter.YawCam` (.yaw (.rotation _outvalue_12)) _asbp_vrcharacter)
                            (bind _camera (`/Game/BP_VRCharacter.Camera` _asbp_vrcharacter))
                            (bind (_returnvalue_roll _returnvalue_pitch _returnvalue_yaw) (`KismetMathLibrary.BreakRotator` (`SceneComponent.K2_GetComponentRotation` _camera)))
                            (`SceneComponent.K2_SetWorldRotation` _camera (`KismetMathLibrary.MakeRotator` (.roll (.rotation _outvalue_12)) (.pitch (.rotation _outvalue_12)) _returnvalue_yaw) false false)))))
                    (`|ExecutionSequence` :!label _label_2
                      (:`then_0`
                        (bind _asblueprint_gi_4 (cast `/Game/BlueprintGI` (`GameplayStatics.GetGameInstance`)))
                        (`self.SwitchSendMethod`
                          (:`Old`
                            (bind _datatick_players (break `/Game/Structs/Struct_DataTick` (`/Game/BlueprintGI.dataTick` _asblueprint_gi_4)))
                            (for (_array_element_2 _array_index) _datatick_players
                              (bind _outvalue_13 (`|GetJsonField` _outjsonobject "from"))
                              (if (`KismetStringLibrary.EqualEqual_StrStr` _outvalue_13 (break `/Game/Structs/Struct_Player` _array_element_2))
                                (bind _outvalue_14 (`|GetJsonField` _outvalue_2 "rotation"))
                                (bind _outvalue_15 (`|GetJsonField` _outvalue_2 "speed"))
                                (bind _outvalue_16 (`|GetJsonField` _outvalue_2 "velocity"))
                                (`KismetArrayLibrary.Array_Set` _datatick_players _array_index (make `/Game/Structs/Struct_Player` (break `/Game/Structs/Struct_Player` _array_element_2) _returnvalue_4 _outvalue_14 _outvalue_15 _outvalue_10 _outvalue_11 _outvalue_12 _outvalue_16 (`.avatar_41_BBB2E1E04B97731DC7F9E486B3740CBB` (break `/Game/Structs/Struct_Player` _array_element_2)))))))
                          (:`New`
                            (bind _dataticknew_players (break `/Game/Structs/NewMethod/Struct_NewDataTick` (`/Game/BlueprintGI.dataTickNew` _asblueprint_gi_4)))
                            (for (_array_element_3 _array_index_2) _dataticknew_players
                              (bind _outvalue_17 (`|GetJsonField` _outjsonobject "from"))
                              (if (`KismetStringLibrary.EqualEqual_StrStr` _outvalue_17 (break `/Game/Structs/NewMethod/Struct_NewPlayer` _array_element_3))
                                (bind _outvalue_18 (`|GetJsonField` _outvalue_2 "rotation"))
                                (bind _outvalue_19 (`|GetJsonField` _outvalue_2 "speed"))
                                (bind _outvalue_20 (`|GetJsonField` _outvalue_2 "velocity"))
                                (bind (_x _y _z) (`KismetMathLibrary.BreakVector3f` _returnvalue_4))
                                (`KismetArrayLibrary.Array_Set` _dataticknew_players _array_index_2 (make `/Game/Structs/NewMethod/Struct_NewPlayer` (break `/Game/Structs/NewMethod/Struct_NewPlayer` _array_element_3) (make `/Game/Structs/Struct_Vector3` (`KismetMathLibrary.FTrunc` _x) (`KismetMathLibrary.FTrunc` _y) (`KismetMathLibrary.FTrunc` _z)) _outvalue_18 _outvalue_19 (stale _outvalue_23) (stale _outvalue_24) (stale _outvalue_25) _outvalue_20 (`.avatar_41_BBB2E1E04B97731DC7F9E486B3740CBB` (break `/Game/Structs/NewMethod/Struct_NewPlayer` _array_element_3)))))))))
                      (:`then_1`
                        (switch `/Game/Enums/Enum_SendMethod` (`/Game/BlueprintGI.SendMethod` (cast `/Game/BlueprintGI` (`GameplayStatics.GetGameInstance`) :!pure true))
                          (:`NewEnumerator0`
                            (`/Game/BP_VRCharacter.TickCICE` (cast `/Game/BP_VRCharacter` (`GameplayStatics.GetPlayerCharacter` 0) :!pure true)))))))
                  (:`New`
                    (bind _outvalue_21 (`|GetJsonField` _outvalue_2 "rotation"))
                    ;[1 1 1] this only happen on client instance (recieving data tick from server)
                    (`|ExecutionSequence`
                      (:`then_0`
                        (bind _outvalue_22 (`|GetJsonField` _outjsonobject "from"))
                        (bind _array_element_4 (`self.FindCharacter` _outvalue_22))
                        (bind _outvalue_23 (`|GetJsonField` _outvalue_2 "MC_Left"))
                        (bind _outvalue_24 (`|GetJsonField` _outvalue_2 "MC_Right"))
                        (bind _outvalue_25 (`|GetJsonField` _outvalue_2 "camera"))
                        (bind _outvalue_26 (`|GetJsonField` _outvalue_2 "speed"))
                        (bind (_x_2 _y_2 _z_2 _w) (break `/Game/Structs/Struct_Rotator` _outvalue_21))
                        (bind (_position _rotator) (break `/Game/Structs/Struct_Transform` _outvalue_23))
                        (bind (_position_2 _rotator_2) (break `/Game/Structs/Struct_Transform` _outvalue_24))
                        (bind (_position_3 _rotator_3) (break `/Game/Structs/Struct_Transform` _outvalue_25))
                        (`/Game/BP_VRCharacter.MoveTo` _array_element_4 _returnvalue_4 (`KismetMathLibrary.Quat_Rotator` (`KismetMathLibrary.MakeQuat` _x_2 _y_2 _z_2 _w)) (`KismetMathLibrary.MakeTransform` (`KismetMathLibrary.MakeVector` (`KismetMathLibrary.Conv_IntToDouble` (break `/Game/Structs/Struct_Vector3` _position)) (`KismetMathLibrary.Conv_IntToDouble` (`.y_8_F4ABCA8649968516F66E4A88C0F8171F` (break `/Game/Structs/Struct_Vector3` _position))) (`KismetMathLibrary.Conv_IntToDouble` (`.z_9_7F80DC244D02B7FD9BD9B7B65B110452` (break `/Game/Structs/Struct_Vector3` _position)))) (`KismetMathLibrary.Quat_Rotator` (`KismetMathLibrary.MakeQuat` (break `/Game/Structs/Struct_Rotator` _rotator) (`.y_5_F4ABCA8649968516F66E4A88C0F8171F` (break `/Game/Structs/Struct_Rotator` _rotator)) (`.z_6_7F80DC244D02B7FD9BD9B7B65B110452` (break `/Game/Structs/Struct_Rotator` _rotator)) (`.w_9_290A57E747B064C11776B4B87C3D3198` (break `/Game/Structs/Struct_Rotator` _rotator))))) (`KismetMathLibrary.MakeTransform` (`KismetMathLibrary.MakeVector` (`KismetMathLibrary.Conv_IntToDouble` (break `/Game/Structs/Struct_Vector3` _position_2)) (`KismetMathLibrary.Conv_IntToDouble` (`.y_8_F4ABCA8649968516F66E4A88C0F8171F` (break `/Game/Structs/Struct_Vector3` _position_2))) (`KismetMathLibrary.Conv_IntToDouble` (`.z_9_7F80DC244D02B7FD9BD9B7B65B110452` (break `/Game/Structs/Struct_Vector3` _position_2)))) (`KismetMathLibrary.Quat_Rotator` (`KismetMathLibrary.MakeQuat` (break `/Game/Structs/Struct_Rotator` _rotator_2) (`.y_5_F4ABCA8649968516F66E4A88C0F8171F` (break `/Game/Structs/Struct_Rotator` _rotator_2)) (`.z_6_7F80DC244D02B7FD9BD9B7B65B110452` (break `/Game/Structs/Struct_Rotator` _rotator_2)) (`.w_9_290A57E747B064C11776B4B87C3D3198` (break `/Game/Structs/Struct_Rotator` _rotator_2))))) (`KismetMathLibrary.MakeTransform` (`KismetMathLibrary.MakeVector` (`KismetMathLibrary.Conv_IntToDouble` (break `/Game/Structs/Struct_Vector3` _position_3)) (`KismetMathLibrary.Conv_IntToDouble` (`.y_8_F4ABCA8649968516F66E4A88C0F8171F` (break `/Game/Structs/Struct_Vector3` _position_3))) (`KismetMathLibrary.Conv_IntToDouble` (`.z_9_7F80DC244D02B7FD9BD9B7B65B110452` (break `/Game/Structs/Struct_Vector3` _position_3)))) (`KismetMathLibrary.Quat_Rotator` (`KismetMathLibrary.MakeQuat` (break `/Game/Structs/Struct_Rotator` _rotator_3) (`.y_5_F4ABCA8649968516F66E4A88C0F8171F` (break `/Game/Structs/Struct_Rotator` _rotator_3)) (`.z_6_7F80DC244D02B7FD9BD9B7B65B110452` (break `/Game/Structs/Struct_Rotator` _rotator_3)) (`.w_9_290A57E747B064C11776B4B87C3D3198` (break `/Game/Structs/Struct_Rotator` _rotator_3))))) _outvalue_26))
                      (:`then_1`
                        (goto _label_2))))))))
          (:`tick`
            (bind _asblueprint_gi_5 (cast `/Game/BlueprintGI` (`GameplayStatics.GetGameInstance`)))
            (switch `/Game/Enums/Enum_UserType` (`/Game/BlueprintGI.role` _asblueprint_gi_5)
              (:`NewEnumerator1`
                (`self.SwitchSendMethod`
                  (:`Old`
                    (bind (_outvalue_27 _returnvalue_5) (`|GetJsonField` _outjsonobject "data"))
                    (bind _output_get (set `/Game/BlueprintGI.dataTick` _outvalue_27 _asblueprint_gi_5))
                    (for _array_element_5 (break `/Game/Structs/Struct_DataTick` _output_get)
                      (`|ExecutionSequence`
                        (:`then_0`
                          (if (`KismetStringLibrary.NotEqual_StrStr` (break `/Game/Structs/Struct_Player` _array_element_5) (`/Game/BP_VRCharacter.socketio_id` (cast `/Game/BP_VRCharacter` (`GameplayStatics.GetPlayerCharacter` 0) :!pure true)))
                            (bind _array_element_6 (`self.FindCharacter` (break `/Game/Structs/Struct_Player` _array_element_5)))
                            (`/Engine/EditorBlueprintResources/StandardMacros.IsValid` _array_element_6
                              (:`Is Valid`
                                (`|ExecutionSequence`
                                  (:`then_0`
                                    (`self.K2_SetActorLocation` _array_element_6 (`.position_14_D25647214EFA4FD416B8F58C500C1DB2` (break `/Game/Structs/Struct_Player` _array_element_5)) false true)
                                    (bind _camera_2 (`/Game/BP_VRCharacter.Camera` _array_element_6))
                                    (bind _rotation (.rotation (`.MC_Left_28_A62E2C6F483EBCEBC04236A64F73CF65` (break `/Game/Structs/Struct_Player` _array_element_5))))
                                    (bind (_returnvalue_roll_2 _returnvalue_pitch_2 _returnvalue_yaw_2) (`KismetMathLibrary.BreakRotator` (`SceneComponent.K2_GetComponentRotation` _camera_2)))
                                    (`SceneComponent.K2_SetWorldRotation` _camera_2 (`KismetMathLibrary.MakeRotator` (.roll _rotation) (.pitch _rotation) _returnvalue_yaw_2) false false)
                                    (set `/Game/BP_VRCharacter.MCL_Location` (.location (`.MC_Left_28_A62E2C6F483EBCEBC04236A64F73CF65` (break `/Game/Structs/Struct_Player` _array_element_5))) _array_element_6)
                                    (set `/Game/BP_VRCharacter.MCL_Rotation` _rotation _array_element_6)
                                    (set `/Game/BP_VRCharacter.MCR_Location` (.location (`.MC_Right_30_BCA9A1E94156C783CD22E6B58E50C15A` (break `/Game/Structs/Struct_Player` _array_element_5))) _array_element_6)
                                    (set `/Game/BP_VRCharacter.MCR_Rotation` (.rotation (`.MC_Right_30_BCA9A1E94156C783CD22E6B58E50C15A` (break `/Game/Structs/Struct_Player` _array_element_5))) _array_element_6)
                                    (set `/Game/BP_VRCharacter.YawCam` (.yaw (.rotation (`.camera_33_F721DC834615C85BC752CF9CEC0AE2A9` (break `/Game/Structs/Struct_Player` _array_element_5)))) _array_element_6))
                                  (:`then_1`
                                    (set `/Game/BP_VRCharacter.currentSpeed` (`.speed_19_5E4ADC3047435F390BF6FA83F1FD22A6` (break `/Game/Structs/Struct_Player` _array_element_5)) _array_element_6)))))))
                        (:`then_1`
                          (bind _indexbreakout (`/Game/Functions/utilities.getPlayerBreakoutRoomCICE` (break `/Game/Structs/Struct_Player` _array_element_5) (cast `/Game/BlueprintGI` (`GameplayStatics.GetGameInstance`) :!pure true)))
                          (if (!= _indexbreakout -1)
                            (bind (_actor _found_) (`/Game/Functions/utilities.getPlayerActor` (break `/Game/Structs/Struct_Player` _array_element_5)))
                            (if _found_
                              (`/Game/BP_VRCharacter.ShowJoinBreakoutButton` _actor))
                            (else
                              (bind (_actor_2 _found__2) (`/Game/Functions/utilities.getPlayerActor` (break `/Game/Structs/Struct_Player` _array_element_5)))
                              (if _found__2
                                (`/Game/BP_VRCharacter.HideJoinBreakoutButton` _actor_2))))))))
                  (:`New`
                    (bind _outvalue_28 (`|GetJsonField` _outjsonobject "data"))
                    (bind _output_get_2 (set `/Game/BlueprintGI.dataTickNew` _outvalue_28 _asblueprint_gi_5))
                    (for _array_element_7 (break `/Game/Structs/NewMethod/Struct_NewDataTick` _output_get_2)
                      (bind _array_element_8 (`self.FindCharacter` (break `/Game/Structs/NewMethod/Struct_NewPlayer` _array_element_7)))
                      (`/Engine/EditorBlueprintResources/StandardMacros.IsValid` _array_element_8
                        (:`Is Valid`
                          (if (not (`Pawn.IsLocallyControlled` _array_element_8))
                            (`|ExecutionSequence`
                              (:`then_0`
                                (if (`KismetStringLibrary.NotEqual_StrStr` (break `/Game/Structs/NewMethod/Struct_NewPlayer` _array_element_7) (`/Game/BP_VRCharacter.socketio_id` (cast `/Game/BP_VRCharacter` (`GameplayStatics.GetPlayerCharacter` 0) :!pure true)))
                                  (`/Game/BP_VRCharacter.MoveTo` _array_element_8 (`KismetMathLibrary.MakeVector` (`KismetMathLibrary.Conv_IntToDouble` (break `/Game/Structs/Struct_Vector3` (`.position_42_D25647214EFA4FD416B8F58C500C1DB2` (break `/Game/Structs/NewMethod/Struct_NewPlayer` _array_element_7)))) (`KismetMathLibrary.Conv_IntToDouble` (`.y_8_F4ABCA8649968516F66E4A88C0F8171F` (break `/Game/Structs/Struct_Vector3` (`.position_42_D25647214EFA4FD416B8F58C500C1DB2` (break `/Game/Structs/NewMethod/Struct_NewPlayer` _array_element_7))))) (`KismetMathLibrary.Conv_IntToDouble` (`.z_9_7F80DC244D02B7FD9BD9B7B65B110452` (break `/Game/Structs/Struct_Vector3` (`.position_42_D25647214EFA4FD416B8F58C500C1DB2` (break `/Game/Structs/NewMethod/Struct_NewPlayer` _array_element_7)))))) (`KismetMathLibrary.Quat_Rotator` (`KismetMathLibrary.MakeQuat` (break `/Game/Structs/Struct_Rotator` (`.rotation_43_642F4CE74C529C7AAB218CB4C1BE8EC3` (break `/Game/Structs/NewMethod/Struct_NewPlayer` _array_element_7))) (`.y_5_F4ABCA8649968516F66E4A88C0F8171F` (break `/Game/Structs/Struct_Rotator` (`.rotation_43_642F4CE74C529C7AAB218CB4C1BE8EC3` (break `/Game/Structs/NewMethod/Struct_NewPlayer` _array_element_7)))) (`.z_6_7F80DC244D02B7FD9BD9B7B65B110452` (break `/Game/Structs/Struct_Rotator` (`.rotation_43_642F4CE74C529C7AAB218CB4C1BE8EC3` (break `/Game/Structs/NewMethod/Struct_NewPlayer` _array_element_7)))) (`.w_9_290A57E747B064C11776B4B87C3D3198` (break `/Game/Structs/Struct_Rotator` (`.rotation_43_642F4CE74C529C7AAB218CB4C1BE8EC3` (break `/Game/Structs/NewMethod/Struct_NewPlayer` _array_element_7)))))) (`KismetMathLibrary.MakeTransform` (`KismetMathLibrary.MakeVector` (`KismetMathLibrary.Conv_IntToDouble` (break `/Game/Structs/Struct_Vector3` (break `/Game/Structs/Struct_Transform` (`.MC_Left_44_A62E2C6F483EBCEBC04236A64F73CF65` (break `/Game/Structs/NewMethod/Struct_NewPlayer` _array_element_7))))) (`KismetMathLibrary.Conv_IntToDouble` (`.y_8_F4ABCA8649968516F66E4A88C0F8171F` (break `/Game/Structs/Struct_Vector3` (break `/Game/Structs/Struct_Transform` (`.MC_Left_44_A62E2C6F483EBCEBC04236A64F73CF65` (break `/Game/Structs/NewMethod/Struct_NewPlayer` _array_element_7)))))) (`KismetMathLibrary.Conv_IntToDouble` (`.z_9_7F80DC244D02B7FD9BD9B7B65B110452` (break `/Game/Structs/Struct_Vector3` (break `/Game/Structs/Struct_Transform` (`.MC_Left_44_A62E2C6F483EBCEBC04236A64F73CF65` (break `/Game/Structs/NewMethod/Struct_NewPlayer` _array_element_7))))))) (`KismetMathLibrary.Quat_Rotator` (`KismetMathLibrary.MakeQuat` (break `/Game/Structs/Struct_Rotator` (`.rotator_6_44BD7BC64D738A76CC489BBFCE35C998` (break `/Game/Structs/Struct_Transform` (`.MC_Left_44_A62E2C6F483EBCEBC04236A64F73CF65` (break `/Game/Structs/NewMethod/Struct_NewPlayer` _array_element_7))))) (`.y_5_F4ABCA8649968516F66E4A88C0F8171F` (break `/Game/Structs/Struct_Rotator` (`.rotator_6_44BD7BC64D738A76CC489BBFCE35C998` (break `/Game/Structs/Struct_Transform` (`.MC_Left_44_A62E2C6F483EBCEBC04236A64F73CF65` (break `/Game/Structs/NewMethod/Struct_NewPlayer` _array_element_7)))))) (`.z_6_7F80DC244D02B7FD9BD9B7B65B110452` (break `/Game/Structs/Struct_Rotator` (`.rotator_6_44BD7BC64D738A76CC489BBFCE35C998` (break `/Game/Structs/Struct_Transform` (`.MC_Left_44_A62E2C6F483EBCEBC04236A64F73CF65` (break `/Game/Structs/NewMethod/Struct_NewPlayer` _array_element_7)))))) (`.w_9_290A57E747B064C11776B4B87C3D3198` (break `/Game/Structs/Struct_Rotator` (`.rotator_6_44BD7BC64D738A76CC489BBFCE35C998` (break `/Game/Structs/Struct_Transform` (`.MC_Left_44_A62E2C6F483EBCEBC04236A64F73CF65` (break `/Game/Structs/NewMethod/Struct_NewPlayer` _array_element_7))))))))) (`KismetMathLibrary.MakeTransform` (`KismetMathLibrary.MakeVector` (`KismetMathLibrary.Conv_IntToDouble` (break `/Game/Structs/Struct_Vector3` (break `/Game/Structs/Struct_Transform` (`.MC_Right_45_BCA9A1E94156C783CD22E6B58E50C15A` (break `/Game/Structs/NewMethod/Struct_NewPlayer` _array_element_7))))) (`KismetMathLibrary.Conv_IntToDouble` (`.y_8_F4ABCA8649968516F66E4A88C0F8171F` (break `/Game/Structs/Struct_Vector3` (break `/Game/Structs/Struct_Transform` (`.MC_Right_45_BCA9A1E94156C783CD22E6B58E50C15A` (break `/Game/Structs/NewMethod/Struct_NewPlayer` _array_element_7)))))) (`KismetMathLibrary.Conv_IntToDouble` (`.z_9_7F80DC244D02B7FD9BD9B7B65B110452` (break `/Game/Structs/Struct_Vector3` (break `/Game/Structs/Struct_Transform` (`.MC_Right_45_BCA9A1E94156C783CD22E6B58E50C15A` (break `/Game/Structs/NewMethod/Struct_NewPlayer` _array_element_7))))))) (`KismetMathLibrary.Quat_Rotator` (`KismetMathLibrary.MakeQuat` (break `/Game/Structs/Struct_Rotator` (`.rotator_6_44BD7BC64D738A76CC489BBFCE35C998` (break `/Game/Structs/Struct_Transform` (`.MC_Right_45_BCA9A1E94156C783CD22E6B58E50C15A` (break `/Game/Structs/NewMethod/Struct_NewPlayer` _array_element_7))))) (`.y_5_F4ABCA8649968516F66E4A88C0F8171F` (break `/Game/Structs/Struct_Rotator` (`.rotator_6_44BD7BC64D738A76CC489BBFCE35C998` (break `/Game/Structs/Struct_Transform` (`.MC_Right_45_BCA9A1E94156C783CD22E6B58E50C15A` (break `/Game/Structs/NewMethod/Struct_NewPlayer` _array_element_7)))))) (`.z_6_7F80DC244D02B7FD9BD9B7B65B110452` (break `/Game/Structs/Struct_Rotator` (`.rotator_6_44BD7BC64D738A76CC489BBFCE35C998` (break `/Game/Structs/Struct_Transform` (`.MC_Right_45_BCA9A1E94156C783CD22E6B58E50C15A` (break `/Game/Structs/NewMethod/Struct_NewPlayer` _array_element_7)))))) (`.w_9_290A57E747B064C11776B4B87C3D3198` (break `/Game/Structs/Struct_Rotator` (`.rotator_6_44BD7BC64D738A76CC489BBFCE35C998` (break `/Game/Structs/Struct_Transform` (`.MC_Right_45_BCA9A1E94156C783CD22E6B58E50C15A` (break `/Game/Structs/NewMethod/Struct_NewPlayer` _array_element_7))))))))) (`KismetMathLibrary.MakeTransform` (`KismetMathLibrary.MakeVector` (`KismetMathLibrary.Conv_IntToDouble` (break `/Game/Structs/Struct_Vector3` (break `/Game/Structs/Struct_Transform` (`.camera_46_F721DC834615C85BC752CF9CEC0AE2A9` (break `/Game/Structs/NewMethod/Struct_NewPlayer` _array_element_7))))) (`KismetMathLibrary.Conv_IntToDouble` (`.y_8_F4ABCA8649968516F66E4A88C0F8171F` (break `/Game/Structs/Struct_Vector3` (break `/Game/Structs/Struct_Transform` (`.camera_46_F721DC834615C85BC752CF9CEC0AE2A9` (break `/Game/Structs/NewMethod/Struct_NewPlayer` _array_element_7)))))) (`KismetMathLibrary.Conv_IntToDouble` (`.z_9_7F80DC244D02B7FD9BD9B7B65B110452` (break `/Game/Structs/Struct_Vector3` (break `/Game/Structs/Struct_Transform` (`.camera_46_F721DC834615C85BC752CF9CEC0AE2A9` (break `/Game/Structs/NewMethod/Struct_NewPlayer` _array_element_7))))))) (`KismetMathLibrary.Quat_Rotator` (`KismetMathLibrary.MakeQuat` (break `/Game/Structs/Struct_Rotator` (`.rotator_6_44BD7BC64D738A76CC489BBFCE35C998` (break `/Game/Structs/Struct_Transform` (`.camera_46_F721DC834615C85BC752CF9CEC0AE2A9` (break `/Game/Structs/NewMethod/Struct_NewPlayer` _array_element_7))))) (`.y_5_F4ABCA8649968516F66E4A88C0F8171F` (break `/Game/Structs/Struct_Rotator` (`.rotator_6_44BD7BC64D738A76CC489BBFCE35C998` (break `/Game/Structs/Struct_Transform` (`.camera_46_F721DC834615C85BC752CF9CEC0AE2A9` (break `/Game/Structs/NewMethod/Struct_NewPlayer` _array_element_7)))))) (`.z_6_7F80DC244D02B7FD9BD9B7B65B110452` (break `/Game/Structs/Struct_Rotator` (`.rotator_6_44BD7BC64D738A76CC489BBFCE35C998` (break `/Game/Structs/Struct_Transform` (`.camera_46_F721DC834615C85BC752CF9CEC0AE2A9` (break `/Game/Structs/NewMethod/Struct_NewPlayer` _array_element_7)))))) (`.w_9_290A57E747B064C11776B4B87C3D3198` (break `/Game/Structs/Struct_Rotator` (`.rotator_6_44BD7BC64D738A76CC489BBFCE35C998` (break `/Game/Structs/Struct_Transform` (`.camera_46_F721DC834615C85BC752CF9CEC0AE2A9` (break `/Game/Structs/NewMethod/Struct_NewPlayer` _array_element_7))))))))) (`.speed_19_5E4ADC3047435F390BF6FA83F1FD22A6` (break `/Game/Structs/NewMethod/Struct_NewPlayer` _array_element_7)))))
                              (:`then_1`
                                (bind _indexbreakout_2 (`/Game/Functions/utilities.getPlayerBreakoutRoomCICE` (break `/Game/Structs/NewMethod/Struct_NewPlayer` _array_element_7) (cast `/Game/BlueprintGI` (`GameplayStatics.GetGameInstance`) :!pure true)))
                                (if (!= _indexbreakout_2 -1)
                                  (`/Game/BP_VRCharacter.ShowJoinBreakoutButton` _array_element_8)
                                  (else
                                    (`/Game/BP_VRCharacter.HideJoinBreakoutButton` _array_element_8))))
                              (:`then_2`
                                (set `/Game/BP_VRCharacter.actualSpeed` (`.speed_19_5E4ADC3047435F390BF6FA83F1FD22A6` (break `/Game/Structs/NewMethod/Struct_NewPlayer` _array_element_7)) _array_element_8)))))
                        (:`Is Not Valid`
                          (`KismetSystemLibrary.PrintString` "CHARACTER NOT FOUND")))))))))
          (:`reply_latency`
            (`self.recieveTimestamp` _outjsonobject)
            (bind _outvalue_29 (`|GetJsonField` _outjsonobject "data"))
            (bind _outvalue_30 (`|GetJsonField` _outvalue_29 "timestamp"))
            (bind _returnvalue_6 (`/Game/Functions/utilities.getUnixTimestamp`))
            (`self.SwitchSendMethod`
              (:`Old`
                (bind _returnvalue_7 (- _returnvalue_6 (`.timestamp_2_8857E3984BCB4678C9C083AE0C4A71DC` (break `/Game/Structs/Struct_Timestamp` _outvalue_30))))
                (`KismetArrayLibrary.Array_Add` (`/Game/BlueprintGI.latencyOld` _asblueprint_gi_2) (make `/Game/Structs/Struct_Latency` (`KismetMathLibrary.Conv_Int64ToInt` _returnvalue_7) _returnvalue_6))
                (bind _output_get_3 (set `/Game/BlueprintGI.totalPingOld` (+ (`/Game/BlueprintGI.totalPingOld` _asblueprint_gi) _returnvalue_7) _asblueprint_gi))
                (bind _result (`/Engine/EditorBlueprintResources/StandardMacros.IncrementInt` (`/Game/BlueprintGI.pingCountOld` _asblueprint_gi))
                  (:`  `
                    (`self.setVariableGI` (`KismetMathLibrary.Conv_Int64ToInt` (/ _output_get_3 _result)) (`KismetMathLibrary.Conv_Int64ToInt` _returnvalue_7)))))
              (:`New`
                (`KismetArrayLibrary.Array_Add` (`/Game/BlueprintGI.latencyNew` _asblueprint_gi_2) (make `/Game/Structs/Struct_Latency` (`KismetMathLibrary.Conv_Int64ToInt` _returnvalue_7) _returnvalue_6))
                (bind _output_get_4 (set `/Game/BlueprintGI.totalPing` (+ (`/Game/BlueprintGI.totalPing` _asblueprint_gi_2) _returnvalue_7) _asblueprint_gi_2))
                (bind _result_2 (`/Engine/EditorBlueprintResources/StandardMacros.IncrementInt` (`/Game/BlueprintGI.pingCount` _asblueprint_gi_2))
                  (:`  `
                    (`self.setVariableGI` (`KismetMathLibrary.Conv_Int64ToInt` (/ _output_get_4 _result_2)) (`KismetMathLibrary.Conv_Int64ToInt` _returnvalue_7)))))))
          (:`draw_location`
            (`self.replyTimestamp` _outjsonobject)
            (bind (_outvalue_31 _returnvalue_8) (`|GetJsonField` _outvalue_2 "location"))
            (bind _outvalue_32 (`|GetJsonField` _outjsonobject "from"))
            (`self.Draw Location` _outvalue_31 _outvalue_32)))))
    (:`NewEnumerator1`
      (goto _label))
    (:`NewEnumerator2`
      (bind _asblueprint_gi_6 (cast `/Game/BlueprintGI` _returnvalue))
      (bind _outvalue_33 (`|GetJsonField` _outjsonobject "socketid"))
      (if (`KismetStringLibrary.EqualEqual_StrStr` _outvalue_33 (`/Game/BlueprintGI.socketid` _asblueprint_gi_6))
        (goto _label)))))

(event `Start`
  (bind _udp (`self.UDP`))
  (`KismetSystemLibrary.PrintString` "UDP STARTED!!")
  (bind _asblueprint_gi (cast `/Game/BlueprintGI` (`GameplayStatics.GetGameInstance`)))
  (`UDPComponent.OpenSendSocket` _udp "127.0.0.1" (`/Game/BlueprintGI.PortUDPserver` _asblueprint_gi))
  (`UDPComponent.OpenReceiveSocket` _udp "0.0.0.0" (`/Game/BlueprintGI.PortUDPclient` _asblueprint_gi)))

(event `self.UDP.OnReceivedBytes`
  (params (Bytes :type "Array of Byte (by ref)") (IPAddress :type String)))

(event `Draw Location`
  (params (NewParam :type "Vector2D Structure") (from :type String))
  (bind _asblueprint_gi (cast `/Game/BlueprintGI` (`GameplayStatics.GetGameInstance`)))
  (bind _whiteboardref (`/Game/BlueprintGI.whiteboardRef` _asblueprint_gi))
  (`/Engine/EditorBlueprintResources/StandardMacros.IsValid` _whiteboardref
    (:`Is Valid`
      (`/Game/WhiteBoard/BP_Whiteboard.Draw On WhiteBoard` _whiteboardref NewParam 0 from))))

(fn `FindCharacter`
  (params (socketid :type String))
  (returns (`Array Element` :type "/Game/BP_VRCharacter Object Reference"))
  (for _array_element (`/Game/BlueprintGI.players_actor` (cast `/Game/BlueprintGI` (`GameplayStatics.GetGameInstance`) :!pure true))
    (if (`KismetStringLibrary.EqualEqual_StrStr` socketid (`/Game/BP_VRCharacter.socketio_id` _array_element))
      (return _array_element))))

(fn `MoveTo`
  (params (Start :type "Vector Structure") (End :type "Vector Structure"))
  (returns (ReturnValue :type "Vector Structure"))
  (return (`|Copy` Start)))

(fn `recieveTimestamp`
  (params (data :type "JsonObjectWrapper Structure"))
  (locals (temp :type "Array of Integer"))
  (bind _outvalue (`|GetJsonField` data "channel"))
  (switch `string` _outvalue
    (:`reply_latency`
      (bind _outvalue_2 (`|GetJsonField` data "data"))
      (bind _outvalue_3 (`|GetJsonField` _outvalue_2 "channel"))
      (bind _returnvalue (`/Game/Functions/utilities.getUnixTimestamp`))
      (bind _outvalue_4 (`|GetJsonField` _outvalue_2 "timestamp"))
      (bind _enum (`/Game/Functions/utilities.StringToEnumChannel` _outvalue_3))
      (bind _asblueprint_gi (cast `/Game/BlueprintGI` (`GameplayStatics.GetGameInstance`)))
      (bind _latency_metaverse (`/Game/BlueprintGI.latency_metaverse` _asblueprint_gi))
      (bind (_value _returnvalue_2) (`BlueprintMapLibrary.Map_Find` _latency_metaverse _enum))
      (if _returnvalue_2
        (bind _output_get (set `local.temp` (break `/Game/Structs/utilities/Struct_LatencyMap` _value)))
        (bind _returnvalue_3 (`KismetMathLibrary.Conv_Int64ToInt` (- _returnvalue (`.timestamp_2_8857E3984BCB4678C9C083AE0C4A71DC` (break `/Game/Structs/Struct_Timestamp` _outvalue_4)))))
        (`KismetArrayLibrary.Array_Add` _output_get _returnvalue_3)
        (`BlueprintMapLibrary.Map_Add` _latency_metaverse _enum (make `/Game/Structs/utilities/Struct_LatencyMap` _output_get))
        (else
          (`BlueprintMapLibrary.Map_Add` _latency_metaverse _enum (make `/Game/Structs/utilities/Struct_LatencyMap` (`|MakeArray` _returnvalue_3))))))))

(fn `Reply Latency`
  (params (NewParam :type "JsonObjectWrapper Structure"))
  (bind _asblueprint_gi (cast `/Game/BlueprintGI` (`GameplayStatics.GetGameInstance`))
    (:`then`
      (if (`|EnumEquality` (`/Game/BlueprintGI.role` _asblueprint_gi) "NewEnumerator0")
        ;[1 1 1] recieve from client, modified the packet add new parameter "replypacket" and send it back to the client (with broadcast, so every client will recieve this packet but only the truly client will read it)
        (`|SetJsonField` NewParam "replypacket" true)
        (bind _outjsonstring (`JsonBlueprintFunctionLibrary.ToString` NewParam))
        (`UDPComponent.EmitBytes` (`self.UDP`) (`CUBlueprintLibrary.Conv_StringToBytes` _outjsonstring))
        (else
          ;[1 1 1] this only execute on client side and checking if has "replypacket" parameter on it and check if this replypacket is truly sent for this client (because this packet is broadcasted to all clients)
          (bind _returnvalue (`JsonBlueprintFunctionLibrary.HasField` NewParam "replypacket"))
          (bind _outvalue (`|GetJsonField` NewParam "nickname"))
          (if (and _returnvalue (`KismetStringLibrary.EqualEqual_StrStr` _outvalue (`EOSGameInstance.nickname` _asblueprint_gi)))
            (bind _outvalue_2 (`|GetJsonField` NewParam "timestamp"))
            (bind _returnvalue_2 (- (`self.get Unix`) _outvalue_2))
            (`KismetSystemLibrary.PrintString` (`KismetStringLibrary.Concat_StrStr` "latency:" (`KismetStringLibrary.Conv_DoubleToString` _returnvalue_2) "ms") true true (struct :`G` 0.66 :`B` 1.0 :`A` 1.0) _returnvalue_2))))
      (return))
    (:`CastFailed`
      (return))))

(fn `replyTimestamp`
  (params (data :type "JsonObjectWrapper Structure"))
  (bind _asblueprint_gi (cast `/Game/BlueprintGI` (`GameplayStatics.GetGameInstance`)))
  (switch `/Game/Enums/Enum_UserType` (`/Game/BlueprintGI.role` _asblueprint_gi)
    (:`NewEnumerator0`
      (bind _outvalue (`|GetJsonField` data "from"))
      (bind _outvalue_2 (`|GetJsonField` data "channel"))
      (bind _returnvalue (`SIOJsonObject.ConstructJsonObject`))
      (bind _outvalue_3 (`|GetJsonField` data "timestamp"))
      (`SIOJsonObject.SetObjectField` _returnvalue "timestamp" (`SIOJLibrary.StructToJsonObject` _outvalue_3))
      (`SIOJsonObject.SetStringField` _returnvalue "channel" _outvalue_2)
      (`/Game/BlueprintGI.ED_SendUnreliableData` _asblueprint_gi _returnvalue "NewEnumerator2" _outvalue "NewEnumerator17"))))

(fn `setVariableGI`
  (params (`average latency` :type Integer) (latency :type Integer))
  (bind _asblueprint_gi (cast `/Game/BlueprintGI` (`GameplayStatics.GetGameInstance`) :!pure true))
  (bind _latencymin (`/Game/BlueprintGI.latencyMin` _asblueprint_gi))
  (bind _latencymax (`/Game/BlueprintGI.latencyMax` _asblueprint_gi))
  (set `/Game/BlueprintGI.latencyAvg` `average latency` _asblueprint_gi)
  (`|VariableSetRef` _latencymin (`KismetMathLibrary.Min` latency _latencymin))
  (`|VariableSetRef` _latencymax (`KismetMathLibrary.Max` latency _latencymax)))

(fn `UserConstructionScript`)