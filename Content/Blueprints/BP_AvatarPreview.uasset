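; Preview character that displays the selected avatar (Brian, Sophie, Jody or Shannon) with a waving animation and name label.
; On BeginPlay it registers with the game instance's avatar-change dispatcher and plays Brian's wave.
; The avatar-change handler stores the choice in the game instance, then swaps skeletal mesh and anim class and plays the matching wave montage.
; It then writes the uppercased enum name to the widget component's text.
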(event `ChangeTextName`
  (params (name :type String))
  (bind _aswd_avatar_name (cast `/Game/Widgets/WD_AvatarName` (`WidgetComponent.GetWidget` (`self.Widget`))))
  (`TextBlock.SetText` (`/Game/Widgets/WD_AvatarName.TextBlock_34` _aswd_avatar_name) (`KismetTextLibrary.Conv_StringToText` name)))

(event `self.ReceiveBeginPlay`
  (bind _asblueprint_gi (cast `/Game/BlueprintGI` (`GameplayStatics.GetGameInstance`)))
  (add `/Game/BlueprintGI.ED_onAvatarChange` _asblueprint_gi (delegate `on Change Avatar`))
  (`self.PlayAnimMontage` "/Game/Characters/Brian/Animation/Waving_brian_Montage.Waving_brian_Montage"))

(event `on Change Avatar`
  (params (avatar :type "/Game/Enums/Enum_Avatar Enum" :default "NewEnumerator0"))
  (set `/Game/BlueprintGI.Avatar` avatar (cast `/Game/BlueprintGI` (`GameplayStatics.GetGameInstance`) :!pure true))
  (`KismetSystemLibrary.PrintString` "Avatar IS CHANGING..." true true (struct :`G` 1.0 :`B` 0.03429 :`A` 1.0))
  (switch `/Game/Enums/Enum_Avatar` avatar
    (:`NewEnumerator0`
      (`SkinnedMeshComponent.SetSkinnedAssetAndUpdate` (`self.Mesh`) "/Game/Characters/Brian/Ch01_nonPBR.Ch01_nonPBR" true)
      (`SkeletalMeshComponent.SetAnimInstanceClass` (`self.Mesh`) "/Game/Characters/Brian/Animation/ABP_PreviewBrian.ABP_PreviewBrian_C")
      (`self.PlayAnimMontage` "/Game/Characters/Brian/Animation/Waving_brian_Montage.Waving_brian_Montage"))
    (:`NewEnumerator1`
      (`SkinnedMeshComponent.SetSkinnedAssetAndUpdate` (`self.Mesh`) "/Game/Characters/Sophie/Sophie.Sophie" true)
      (`SkeletalMeshComponent.SetAnimInstanceClass` (`self.Mesh`) "/Game/Characters/Sophie/Animation/ABP_PreviewSophie.ABP_PreviewSophie_C")
      (`self.PlayAnimMontage` "/Game/Characters/Sophie/Animation/Waving_sophie_Montage.Waving_sophie_Montage"))
    (:`NewEnumerator2`
      (`SkinnedMeshComponent.SetSkinnedAssetAndUpdate` (`self.Mesh`) "/Game/Characters/Jody/Jody.Jody" true)
      (`SkeletalMeshComponent.SetAnimInstanceClass` (`self.Mesh`) "/Game/Characters/Jody/Animation/ABP_PreviewJody.ABP_PreviewJody_C")
      (`self.PlayAnimMontage` "/Game/Characters/Jody/Animation/Waving_Jody_Montage.Waving_Jody_Montage"))
    (:`NewEnumerator3`
      (`SkinnedMeshComponent.SetSkinnedAssetAndUpdate` (`self.Mesh`) "/Game/Characters/Shannon/Shannon.Shannon" true)
      (`SkeletalMeshComponent.SetAnimInstanceClass` (`self.Mesh`) "/Game/Characters/Shannon/Animation/ABP_PreviewShannon.ABP_PreviewShannon_C")
      (`self.PlayAnimMontage` "/Game/Characters/Shannon/Animation/Waving_shannon_Montage.Waving_shannon_Montage")))
  (`self.ChangeTextName` (`KismetStringLibrary.ToUpper` (`|GetEnumeratorNameAsString` avatar))))

(event `/Game/Interface/Interface.onChangeAvatar`
  (params (avatar :type "/Game/Enums/Enum_Avatar Enum" :default "NewEnumerator0")))

(fn `UserConstructionScript`)