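; BP_TextNearJoystick is a VR hint actor that shows floating text by the player's right motion controller.
; On BeginPlay in Avatar Selection Map, it teleports to that controller, attaches to it and sets its WD_TextNearJoystick widget to explain changing avatar with the joystick.
; Every Tick it rotates the widget to face the VR character's camera, whichever level is loaded.
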(event `self.ReceiveBeginPlay`
  (bind _returnvalue (`GameplayStatics.GetCurrentLevelName` true))
  (switch `string` _returnvalue
    (:`AvatarSelectionMap`
      (bind _asbp_vrcharacter (cast `/Game/BP_VRCharacter` (`GameplayStatics.GetPlayerCharacter` 0)))
      (bind _motioncontroller_r (`/Game/BP_VRCharacter.MotionController_R` _asbp_vrcharacter))
      (`self.K2_SetActorLocation` self (`SceneComponent.K2_GetComponentLocation` _motioncontroller_r) false true)
      (`self.K2_AttachToComponent` self _motioncontroller_r "None" "KeepRelative" "KeepRelative" "KeepRelative" true)
      (bind _aswd_text_near_joystick (cast `/Game/Widgets/WD_TextNearJoystick` (`WidgetComponent.GetWidget` (`self.Widget`))))
      (`TextBlock.SetText` (`/Game/Widgets/WD_TextNearJoystick.TextBlock_34` _aswd_text_near_joystick) "move joystick to change avatar"))))

(event `self.ReceiveTick`
  (params (DeltaSeconds :type "Float (single-precision)"))
  (bind _widget (`self.Widget`))
  (bind _asbp_vrcharacter (cast `/Game/BP_VRCharacter` (`GameplayStatics.GetPlayerCharacter` 0)))
  (`SceneComponent.K2_SetWorldRotation` _widget (`KismetMathLibrary.FindLookAtRotation` (`SceneComponent.K2_GetComponentLocation` _widget) (`SceneComponent.K2_GetComponentLocation` (`/Game/BP_VRCharacter.Camera` _asbp_vrcharacter))) false false))

(fn `UserConstructionScript`)