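; BP_Menu is a VR menu panel actor that appears in front of the player's camera on demand.
; On BeginPlay it picks the Plane's material by level name, with a separate one for Avatar Selection Map, and binds to BP_VRCharacter's OnChangeMenuHTP event.
; Showing teleports it 150 units ahead of the camera, facing it, while hiding moves it to a far fixed spot and hides it.
; Older widget-texture and toggle logic is left disconnected.
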(event `self.ReceiveBeginPlay`
  (bind _plane (`self.Plane`))
  (`|ExecutionSequence`
    (:`then_0`
      (bind _returnvalue (`GameplayStatics.GetCurrentLevelName` true))
      (switch `string` _returnvalue
        (:`Default`
          (`PrimitiveComponent.SetMaterial` _plane 0 "/Game/Materials/M_PlaneTexture2.M_PlaneTexture2"))
        (:`AvatarSelectionMap`
          (`PrimitiveComponent.SetMaterial` _plane 0 "/Game/Materials/M_PlaneTexture1.M_PlaneTexture1"))))
    (:`then_1`
      (add `/Game/BP_VRCharacter.onChangeMenuHTP` (cast `/Game/BP_VRCharacter` (`GameplayStatics.GetPlayerCharacter` 0) :!pure true) (delegate `onChangeStateHTP`)))))

(event `self.ReceiveTick`
  (params (DeltaSeconds :type "Float (single-precision)")))

(event `onChangeStateHTP`
  (params (show :type Boolean))
  (if show
    (`self.Spawn`)
    (else
      (`self.Hide`))))

(event `Spawn`
  (bind _camera (`/Game/BP_VRCharacter.Camera` (cast `/Game/BP_VRCharacter` (`GameplayStatics.GetPlayerCharacter` 0) :!pure true)))
  (bind _returnvalue (`SceneComponent.K2_GetComponentLocation` _camera))
  (bind _returnvalue_2 (+ (* (`SceneComponent.GetForwardVector` _camera) 150.0) _returnvalue))
  (`self.K2_SetActorLocation` _returnvalue_2 false true)
  (`self.K2_SetActorRotation` (`KismetMathLibrary.FindLookAtRotation` _returnvalue_2 _returnvalue))
  (`self.SetActorHiddenInGame` false))

(event `Hide`
  (`self.K2_SetActorLocation` (0.0 3000.0 3000.0) false true)
  (`self.SetActorHiddenInGame` true))

(fn `UserConstructionScript`)