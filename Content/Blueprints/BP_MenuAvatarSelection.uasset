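; BP_MenuAvatarSelection is an avatar selection menu actor that follows the VR player's view.
; A looping half-second timer replays a timeline that eases it to a point 300 units along the camera's forward vector, turning only its yaw toward the camera.
; A BP_VRPlayer button binding calls StopFollow to clear the timer, but the Handler assignment is disconnected, so that timer's handle is never stored.
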(event `StopFollow`
  (`KismetSystemLibrary.PrintString` "STOP FOLLOW" true true (struct :`R` 1.0 :`G` 0.058244 :`A` 1.0) 5.0)
  (`KismetSystemLibrary.K2_ClearAndInvalidateTimerHandle` (`self.Handler`)))

(event `self.ReceiveBeginPlay`
  (bind _returnvalue (`KismetSystemLibrary.K2_SetTimerDelegate` (delegate `FollowCamera`) 0.5 true))
  (bind _asbp_vrplayer (cast `/Game/Blueprints/BP_VRPlayer` (`GameplayStatics.GetPlayerPawn` 0)))
  (add `/Game/Blueprints/BP_VRPlayer.ED_XButton` _asbp_vrplayer (delegate `StopFollow`)))

(event `FollowCamera`
  (bind (_returnvalue_roll _returnvalue_pitch _returnvalue_yaw) (`KismetMathLibrary.BreakRotator` (`self.K2_GetActorRotation` self)))
  (bind _asbp_vrplayer (cast `/Game/Blueprints/BP_VRPlayer` (`GameplayStatics.GetPlayerPawn` 0)))
  (set `self.oldYaw` _returnvalue_yaw)
  (bind _camera (`/Game/Blueprints/BP_VRPlayer.Camera` _asbp_vrplayer))
  (bind _returnvalue (`SceneComponent.K2_GetComponentLocation` _camera))
  (bind _returnvalue_2 (+ _returnvalue (* (`KismetMathLibrary.Normal` (`KismetMathLibrary.GetForwardVector` (`SceneComponent.K2_GetComponentRotation` _camera))) 300.0)))
  (bind (_returnvalue_roll_2 _returnvalue_pitch_2 _returnvalue_yaw_2) (`KismetMathLibrary.BreakRotator` (`KismetMathLibrary.FindLookAtRotation` _returnvalue_2 _returnvalue)))
  (set `self.newYaw` _returnvalue_yaw_2)
  (set `self.oldPosition` (`self.K2_GetActorLocation` self))
  (set `self.newPosition` _returnvalue_2)
  (bind (_direction _alpha) (`Timeline|Lerp` :!via `PlayFromStart`)
    (:`Update`
      (`self.K2_SetActorLocation` self (`KismetMathLibrary.VLerp` (`self.oldPosition`) (`self.newPosition`) _alpha) false false)
      (bind (_returnvalue_roll_3 _returnvalue_pitch_3 _returnvalue_yaw_3) (`KismetMathLibrary.BreakRotator` (`KismetMathLibrary.RLerp` (`KismetMathLibrary.MakeRotator` 0.0 0.0 (`self.oldYaw`)) (`KismetMathLibrary.MakeRotator` 0.0 0.0 (`self.newYaw`)) _alpha true)))
      (`self.K2_SetActorRotation` self (`KismetMathLibrary.MakeRotator` 0.0 0.0 _returnvalue_yaw_3) false))))

(fn `UserConstructionScript`)