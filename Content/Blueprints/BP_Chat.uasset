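; BP_Chat is an actor that floats in front of the VR player while the character's ShowVRKeyboard flag is set.
; Each Tick it polls BP_VRCharacter, teleporting to a fixed distance along the camera's forward vector at camera height and turning toward the camera.
; The look-at starts from the unflattened forward point, so the actor tilts with head pitch.
; When the flag is off, it hides and parks at a far-off location.
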(event `self.ReceiveTick`
  (params (DeltaSeconds :type "Float (single-precision)"))
  (bind _asbp_vrcharacter (cast `/Game/BP_VRCharacter` (`GameplayStatics.GetPlayerCharacter` 0)))
  (if (not (`/Game/BP_VRCharacter.showVRKeyboard` _asbp_vrcharacter))
    (`self.SetActorHiddenInGame` true)
    (`self.K2_SetActorLocation` (0.0 3000.0 3000.0) false true)
    (else
      (`self.SetActorHiddenInGame` false)
      (bind _camera (`/Game/BP_VRCharacter.Camera` _asbp_vrcharacter))
      (bind _returnvalue (`SceneComponent.K2_GetComponentLocation` _camera))
      (bind (_returnvalue_x _returnvalue_y _returnvalue_z) (`KismetMathLibrary.BreakVector` (+ _returnvalue (* (`SceneComponent.GetForwardVector` _camera) 300))))
      (bind (_returnvalue_x_2 _returnvalue_y_2 _returnvalue_z_2) (`KismetMathLibrary.BreakVector` (`SceneComponent.K2_GetComponentLocation` _camera)))
      (`self.K2_SetActorLocation` (`KismetMathLibrary.MakeVector` _returnvalue_x _returnvalue_y _returnvalue_z_2) false true)
      (`self.K2_SetActorRotation` (`KismetMathLibrary.FindLookAtRotation` (`KismetMathLibrary.MakeVector` _returnvalue_x _returnvalue_y _returnvalue_z) _returnvalue)))))

(fn `UserConstructionScript`)